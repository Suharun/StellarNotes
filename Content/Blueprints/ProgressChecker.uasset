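; ProgressChecker drives the space game's scripted tutorial and tracks player progress: coins, distance travelled and speed upgrades.
; Tick clears read text boxes and advances the intro, then gates music, shockwave and completion steps through boolean flags.
; Externally triggered events show tutorial and milestone lines through one typewriter widget at a time, using DoOnce nodes that reset if no box appears.
; After the tutorial, Tick applies speed upgrades and accumulates distance.
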(event Custom|AddCoins
  (params (Value :type Float%20%28single-precision%29))
  (if (and (Math|Boolean|Equal(Boolean) (Variables|Upgrades|GetMoneyUpgrade) false) (>= (Variables|Default|GetCurrentGold) (Variables|Default|GetMaxGold)))
    (Variables|Default|SetCurrentGold (+ (Variables|Default|GetMaxGold) 25.0))
    (CallFunction|MoreCoinsText)
    (else
      (bind _output_get (Variables|Default|SetCurrentGold (+ Value (Variables|Default|GetCurrentGold))))
      (if (>= _output_get 1e+04)
        (CallFunction|10000CoinsCollectedText))
      (Variables|Default|SetTotalGoldCollected (+ _output_get (Variables|Default|GetTotalGoldCollected))))))

(event Custom|CoinTextBox
  ;[1 1 1] Dialogue Section
  (Utilities|FlowControl|DoOnce false
    (:Completed
      (Utilities|FlowControl|Delay 0.3)
      (CallFunction|BasicCreateTextBox "Hey it's a Coin! That could be useful. 
I wonder if there is a Shop somewhere." (Variables|TextBox|GetPlayerImage)))))

(event Custom|ShopSeenText
  ;[1 1 1] Dialogue Section
  (Utilities|IsValid (Variables|TextBox|GetTextBox)
    (:Is%20Not%20Valid
      (Utilities|FlowControl|DoOnce false :!label _label
        (:Completed
          (CallFunction|BasicCreateTextBox "Oh nice. Another Shop. Perfecto. 
Time to spend all this \"hard-earned\" cash. 
Haha get it? It's because it comes from Rocks. 
I am Hilarious." (Variables|TextBox|GetPlayerImage))
          (Utilities|IsValid (Variables|TextBox|GetTextBox)
            (:Is%20Not%20Valid
              (goto _label Reset))))))))

(event Custom|MusicText
  ;[1 1 1] Dialogue Section
  (Utilities|IsValid (Variables|TextBox|GetTextBox)
    (:Is%20Not%20Valid
      (Utilities|FlowControl|DoOnce false :!label _label
        (:Completed
          (CallFunction|BasicCreateTextBox "Oh Perfect Timing!  
Here is your ride. This will get you moving." (Variables|TextBox|GetAdamImage))
          (Utilities|IsValid (Variables|TextBox|GetTextBox)
            (:Is%20Valid
              (Variables|PorgressionChecks|SetMusicCompleted? true))
            (:Is%20Not%20Valid
              (goto _label Reset))))))))

(event Custom|DisengageText
  ;[1 1 1] Dialogue Section
  (Utilities|IsValid (Variables|TextBox|GetTextBox)
    (:Is%20Not%20Valid
      (Utilities|FlowControl|DoOnce false :!label _label
        (:Completed
          (CallFunction|BasicCreateTextBox "Oh right I forgot to mention. 
If you have music equipped, you can create a shockwave  
to destroy obstacles by pressing Space." (Variables|TextBox|GetAdamImage))
          (Utilities|IsValid (Variables|TextBox|GetTextBox)
            (:Is%20Valid
              (Variables|PorgressionChecks|SetDisengageCompleted? true))
            (:Is%20Not%20Valid
              (goto _label Reset))))))))

(event Custom|20%20Musics%20Found%20Text
  ;[1 1 1] Dialogue Section
)

(event Custom|5000m%20Moved%20Text
  ;[1 1 1] Dialogue Section
  (Utilities|IsValid (Variables|TextBox|GetTextBox)
    (:Is%20Not%20Valid
      (Utilities|FlowControl|DoOnce false :!label _label
        (:Completed
          (CallFunction|BasicCreateTextBox "Thank god I'm floating 10 000 miles and not walking them." (Variables|TextBox|GetPlayerImage))
          (Utilities|IsValid (Variables|TextBox|GetTextBox)
            (:Is%20Valid
              (Variables|PorgressionChecks|Set5000m%20Moved? true))
            (:Is%20Not%20Valid
              (goto _label Reset))))))))

(event Custom|10%20Musics%20Found%20Text
  ;[1 1 1] Dialogue Section
)

(event Custom|10000%20Coins%20Collected%20Text
  ;[1 1 1] Dialogue Section
  (Utilities|IsValid (Variables|TextBox|GetTextBox)
    (:Is%20Not%20Valid
      (Utilities|FlowControl|DoOnce false :!label _label
        (:Completed
          (CallFunction|BasicCreateTextBox "Ahahahahah! 
I HAVE SO MUCH MONEYYYY!" (Variables|TextBox|GetPlayerImage))
          (Utilities|IsValid (Variables|TextBox|GetTextBox)
            (:Is%20Valid
              (Variables|PorgressionChecks|Set10%20000%20Coins%20Found? true))
            (:Is%20Not%20Valid
              (goto _label Reset))))))))

(event Custom|DestroyTextBox
  ;[1 1 1] Dialogue Section
  (Utilities|IsValid (Variables|TextBox|GetTextBox)
    (:Is%20Valid
      (if (Variables|/Game/Widgets/TypeWriterWidget.TypeWriterWidget_C|GetTextRead (Variables|TextBox|GetTextBox))
        (Utilities|FlowControl|Delay (+ (Math|Conversions|ToFloat(Byte) (Variables|TextBox|GetTextSpeed)) 1.0))
        (Widget|RemovefromParent (Variables|TextBox|GetTextBox))
        (Variables|TextBox|SetTextBox 0)
        (if (not (Variables|PorgressionChecks|GetIntroCompleted?))
          (Variables|TextBox|SetIndex (+ (Variables|TextBox|GetIndex) 1)))))))

(event Custom|MoreCoins%20Text
  (Utilities|IsValid (Variables|TextBox|GetTextBox)
    (:Is%20Not%20Valid
      (Utilities|FlowControl|DoOnce false :!label _label
        (:Completed
          (CallFunction|BasicCreateTextBox "Drat, I can't carry anymore Gold. 
Maybe I can buy a bigger Coin Pouch." (Variables|TextBox|GetPlayerImage))
          (Utilities|IsValid (Variables|TextBox|GetTextBox)
            (:Is%20Not%20Valid
              (goto _label Reset))))))))

(event Custom|Intro%20TextBox
  (params (Index :type Integer))
  ;[1 1 1] Dialogue Section
  (CallFunction|BasicCreateTextBox (Utilities|Array|Get(acopy) (Variables|TextBox|GetIntroText) Index) (Variables|TextBox|GetAdamImage)))

(event Custom|ZoomInText
  ;[1 1 1] Dialogue Section
  (Utilities|IsValid (Variables|TextBox|GetTextBox)
    (:Is%20Not%20Valid
      (Utilities|FlowControl|DoOnce false :!label _label
        (:Completed
          (Utilities|FlowControl|Delay 0.3)
          (CallFunction|BasicCreateTextBox "Cool.  
Now Zoom Out by pressing the Down Arrow." (Variables|TextBox|GetAdamImage))
          (Utilities|IsValid (Variables|TextBox|GetTextBox)
            (:Is%20Valid
              (Variables|PorgressionChecks|SetPlayerZoomedOut? true))
            (:Is%20Not%20Valid
              (goto _label Reset))))))))

(event Custom|ShopDiscoveredText
  ;[1 1 1] Dialogue Section
  (Utilities|IsValid (Variables|TextBox|GetTextBox)
    (:Is%20Not%20Valid
      (Utilities|FlowControl|DoOnce false :!label _label
        (:Completed
          (CallFunction|BasicCreateTextBox "Would you look at that. That seems to be a Shop. 
A Shop... In Space... What are the odds." (Variables|TextBox|GetPlayerImage))
          (Utilities|IsValid (Variables|TextBox|GetTextBox)
            (:Is%20Valid
              (Variables|PorgressionChecks|SetShopDiscovered? true))
            (:Is%20Not%20Valid
              (goto _label Reset))))))))

(event Custom|RotateLeftText
  ;[1 1 1] Dialogue Section
  (Utilities|IsValid (Variables|TextBox|GetTextBox)
    (:Is%20Not%20Valid
      (Utilities|FlowControl|DoOnce false :!label _label
        (:Completed
          (Utilities|FlowControl|Delay 0.3)
          (CallFunction|BasicCreateTextBox "Awesome.  
Now rotate right by pressing D or the Right Arrow" (Variables|TextBox|GetAdamImage))
          (Utilities|IsValid (Variables|TextBox|GetTextBox)
            (:Is%20Valid
              (Variables|PorgressionChecks|SetPlayerRotatedLeft? true))
            (:Is%20Not%20Valid
              (goto _label Reset))))))))

(event Custom|RotateRightText
  ;[1 1 1] Dialogue Section
  (Utilities|IsValid (Variables|TextBox|GetTextBox)
    (:Is%20Not%20Valid
      (Utilities|FlowControl|DoOnce false :!label _label
        (:Completed
          (Utilities|FlowControl|Delay 0.3)
          (CallFunction|BasicCreateTextBox "Rotations Complete. 
Now Zoom In by Pressing the Up Arrow" (Variables|TextBox|GetAdamImage))
          (Utilities|IsValid (Variables|TextBox|GetTextBox)
            (:Is%20Valid
              (Variables|PorgressionChecks|SetPlayerRotateCompleted? true))
            (:Is%20Not%20Valid
              (goto _label Reset))))))))

(event Custom|Shockwave%20Text
  ;[1 1 1] Dialogue Section
  (Utilities|IsValid (Variables|TextBox|GetTextBox)
    (:Is%20Not%20Valid
      (Utilities|FlowControl|DoOnce false :!label _label
        (:Completed
          (CallFunction|BasicCreateTextBox "Hell Yes! I love shockwaves. 
Oh Right, it does kill your ride. Another one should come soon 
so no worries. Best of luck!" (Variables|TextBox|GetAdamImage))
          (Utilities|IsValid (Variables|TextBox|GetTextBox)
            (:Is%20Valid
              (Variables|PorgressionChecks|SetShockwaveCompleted? true))
            (:Is%20Not%20Valid
              (goto _label Reset))))))))

(event Custom|ZoomOutText
  ;[1 1 1] Dialogue Section
  (Utilities|IsValid (Variables|TextBox|GetTextBox)
    (:Is%20Not%20Valid
      (Utilities|FlowControl|DoOnce false :!label _label
        (:Completed
          (Utilities|FlowControl|Delay 0.3)
          (CallFunction|BasicCreateTextBox "Congratulations. This should help you navigate." (Variables|TextBox|GetAdamImage))
          (Utilities|IsValid (Variables|TextBox|GetTextBox)
            (:Is%20Valid
              (Variables|PorgressionChecks|SetZoomCompleted? true))
            (:Is%20Not%20Valid
              (goto _label Reset))))))))

(event EventBeginPlay
  (bind _outactors (Actor|GetAllActorsOfClass "/Game/Blueprints/MusicMobs/MusicBase.MusicBase_C"))
  (for _array_element _outactors
    (if (Variables|/Game/Blueprints/MusicMobs/MusicBase.MusicBase_C|GetIsTutorial _array_element)
      (Variables|Default|SetMusicTut _array_element)))
  (Variables|TextBox|SetTextBox 0)
  (Variables|TextBox|SetIntroText (Utilities|Array|MakeArray "Oh Goodness.  
It seems you are lost in space." "Do you remember how to navigate around?" "Hmmmm ....  
It looks like you have forgotten...." "Okay, let's get you back up to speed." "First off let's get you rotating again.  
Press A or the Left Arrow to turn Left."))
  (Utilities|IsValid (Variables|Default|GetPlayer)
    (:Is%20Valid
      (Utilities|FlowControl|Delay 5.0)
      (CallFunction|IntroTextBox (Variables|TextBox|GetIndex)))))

(event EventTick
  (params (DeltaSeconds :type Float%20%28single-precision%29))
  (bind _musictut (Variables|Default|GetMusicTut))
  (bind _player (Variables|Default|GetPlayer))
  (CallFunction|DestroyTextBox)
  (if (Variables|PorgressionChecks|GetTutorialCompleted?)
    (CallFunction|SpeedManagement)
    (if (or (Variables|/Game/2DSideScrollerBP/Blueprints/Player.Player_C|GetCanMove (Variables|Default|GetPlayer)) (Variables|Upgrades|GetMovementUpgrade))
      (Utilities|FlowControl|Delay 0.3)
      (bind _output_get (Variables|Default|SetTotalDistance (+ (Variables|Default|GetTotalDistance) (Variables|Default|GetDistanceIncrease))))
      (Development|PrintString (Utilities|String|ToString(Float) _output_get))
      (if (and (>= _output_get 5e+03) (Math|Boolean|Equal(Boolean) (Variables|PorgressionChecks|Get5000m%20Moved?) false))
        (CallFunction|5000mMovedText)))
    (elif (Variables|PorgressionChecks|GetIntroCompleted?)
      (if (Variables|PorgressionChecks|GetZoomCompleted?)
        (if (Variables|PorgressionChecks|GetMusicCompleted?)
          (if (Variables|PorgressionChecks|GetDisengageCompleted?)
            (if (Variables|PorgressionChecks|GetShockwaveCompleted?)
              (Variables|PorgressionChecks|SetTutorialCompleted? true)
              (else
                (Transformation|SetActorLocation _player "0,-60.000000, 0" false false)
                (if (<= (Variables|/Game/2DSideScrollerBP/Blueprints/Player.Player_C|GetRingScaleIndex _player) 0)
                  (CallFunction|ShockwaveText))))
            (else
              (Utilities|IsValid (Utilities|Array|Get(acopy) (Variables|/Game/2DSideScrollerBP/Blueprints/Player.Player_C|GetRings _player))
                (:Is%20Valid
                  (Utilities|FlowControl|Delay 1.0)
                  (CallFunction|DisengageText)))))
          (else
            (Utilities|IsValid _musictut
              (:Is%20Valid
                (Variables|/Game/Blueprints/MusicMobs/MusicBase.MusicBase_C|SetIsMovable _musictut true)
                (Utilities|FlowControl|Delay 0.8)
                (CallFunction|MusicText))))))
      (elif (>= (Variables|TextBox|GetIndex) 5)
        (Utilities|FlowControl|Delay 0.5)
        (Variables|PorgressionChecks|SetIntroCompleted? true)
        (else
          (Utilities|IsValid (Variables|TextBox|GetTextBox)
            (:Is%20Not%20Valid
              (CallFunction|IntroTextBox (Variables|TextBox|GetIndex)))))))))

(fn ConstructionScript)

(fn BasicCreateTextBox
  (params (Text :type String) (Image :type Paper%20Sprite%20Object%20Reference))
  (Utilities|IsValid (Variables|TextBox|GetTextBox)
    (:Is%20Not%20Valid
      (bind _returnvalue (UserInterface|CreateWidget "/Game/Widgets/TypeWriterWidget.TypeWriterWidget_C" (Game|GetPlayerController 0) Text Image))
      (UserInterface|Viewport|AddtoViewport _returnvalue 0)
      (Variables|TextBox|SetTextBox _returnvalue))))

(fn SpeedManagement
  (bind _player (Variables|Default|GetPlayer))
  (if (Variables|Upgrades|GetSpeedUpgrade1)
    (Variables|/Game/2DSideScrollerBP/Blueprints/Player.Player_C|SetMovementSpeed _player 3e+01)
    (Variables|Default|SetDistanceIncrease 2.0)
    (if (Variables|Upgrades|GetSpeedUpgrade2)
      (Variables|/Game/2DSideScrollerBP/Blueprints/Player.Player_C|SetMovementSpeed _player 6e+01)
      (Variables|Default|SetDistanceIncrease 3.0))))