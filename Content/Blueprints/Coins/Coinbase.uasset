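; Base coin pickup actor that adds its Value to the game's coin count when the player touches it.
; On BeginPlay it caches the first ProgressChecker and Player actors found in the level, though the Player reference is not used afterwards.
; When a Player overlaps its Sphere, it passes Value to the ProgressChecker's AddCoins and destroys itself.
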(event OnComponentBeginOverlap(Sphere)
  (params (OverlappedComponent :type Primitive%20Component%20Object%20Reference) (OtherActor :type Actor%20Object%20Reference) (OtherComp :type Primitive%20Component%20Object%20Reference) (OtherBodyIndex :type Integer) (bFromSweep :type Boolean) (SweepResult :type Hit%20Result%20Structure%20%28by%20ref%29))
  (bind _asplayer (Utilities|Casting|CastToPlayer OtherActor))
  (Utilities|IsValid _asplayer
    (:Is%20Valid
      (Default|AddCoins (Variables|Default|GetPCRef) (Variables|Default|GetValue))
      (Actor|DestroyActor))))

(event EventBeginPlay
  (bind _outactors (Actor|GetAllActorsOfClass "/Game/Blueprints/ProgressChecker.ProgressChecker_C"))
  (Utilities|IsValid (Utilities|Array|Get(acopy) _outactors)
    (:Is%20Valid
      (Variables|Default|SetPCRef (Utilities|Array|Get(acopy) _outactors)))
    (:Is%20Not%20Valid
      _))
  (bind _outactors_2 (Actor|GetAllActorsOfClass "/Game/2DSideScrollerBP/Blueprints/Player.Player_C"))
  (Utilities|IsValid (Utilities|Array|Get(acopy) _outactors_2)
    (:Is%20Valid
      (Variables|Default|SetPlayer (Utilities|Array|Get(acopy) _outactors_2)))))

(event Collision|EventActorBeginOverlap
  (params (OtherActor :type Actor%20Object%20Reference)))

(event EventTick
  (params (DeltaSeconds :type Float%20%28single-precision%29)))

(fn ConstructionScript)