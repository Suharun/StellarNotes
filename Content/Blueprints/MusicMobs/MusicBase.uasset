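; MusicBase is a music mob actor that, when movable, homes in on the player and is collected into their inventory on contact.
; BeginPlay caches the first Player, and Tick steers ProjectileMovement toward it at MovementSpeed.
; Capsule overlap with a Player stops movement, starts the Dissapear flipbook and sets IsAttached.
; From frame 3 of playback, Tick hides it, disables collision and calls AddToInv, with no guard against repeats.
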(event OnComponentBeginOverlap(Capsule)
  (params (OverlappedComponent :type Primitive%20Component%20Object%20Reference) (OtherActor :type Actor%20Object%20Reference) (OtherComp :type Primitive%20Component%20Object%20Reference) (OtherBodyIndex :type Integer) (bFromSweep :type Boolean) (SweepResult :type Hit%20Result%20Structure%20%28by%20ref%29))
  (bind _asplayer (Utilities|Casting|CastToPlayer OtherActor))
  (Utilities|IsValid _asplayer
    (:Is%20Valid
      (Components|Movement|StopMovementImmediately (Variables|Default|GetProjectileMovement))
      (Sprite|SetFlipbook (Variables|Default|GetPaperFlipbook) "/Game/Anims/Dissapear.Dissapear")
      (Variables|Default|SetIsAttached true))))

(event EventBeginPlay
  (bind _outactors (Actor|GetAllActorsOfClass "/Game/2DSideScrollerBP/Blueprints/Player.Player_C"))
  (Utilities|IsValid (Utilities|Array|Get(acopy) _outactors)
    (:Is%20Valid
      (Variables|Default|SetPlayerRef (Utilities|Array|Get(acopy) _outactors))
      (Variables|Default|SetIsAttached false))))

(event Collision|EventActorBeginOverlap
  (params (OtherActor :type Actor%20Object%20Reference)))

(event EventTick
  (params (DeltaSeconds :type Float%20%28single-precision%29))
  (bind _playerref (Variables|Default|GetPlayerRef))
  (Utilities|IsValid _playerref
    (:Is%20Valid
      (if (Variables|Default|GetIsAttached)
        (if (>= (Class|PaperFlipbookComponent|GetPlaybackPositioninFrames (Variables|Default|GetPaperFlipbook)) 3)
          (Rendering|SetVisibility (Variables|Default|GetDefaultSceneRoot) false true)
          (Collision|SetCollisionEnabled (Variables|Default|GetCapsule) "NoCollision")
          (Default|AddtoInv (Variables|Default|GetPlayerRef) self))
        (elif (Variables|Default|GetIsMovable)
          (Variables|/Script/Engine.MovementComponent|SetVelocity (Variables|Default|GetProjectileMovement) (* (Math|Vector|Normalize (- (Transformation|GetWorldLocation (Variables|/Game/2DSideScrollerBP/Blueprints/Player.Player_C|GetScene _playerref)) (Transformation|GetActorLocation))) (Variables|Default|GetMovementSpeed))))))))

(fn ConstructionScript)