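; LimitBP is an actor that shows a limit warning widget when the player leaves its collision volume.
; On BeginPlay it creates a LimitWidget for the first player controller, adds it to the viewport and hides it.
; The collision component's end overlap with a Player makes the widget visible, and the actor's begin overlap with a Player hides it again.
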(event OnComponentEndOverlap(CollisionComponent)
  (params (OverlappedComponent :type Primitive%20Component%20Object%20Reference) (OtherActor :type Actor%20Object%20Reference) (OtherComp :type Primitive%20Component%20Object%20Reference) (OtherBodyIndex :type Integer))
  (Utilities|Casting|CastToPlayer OtherActor)
  (Widget|SetVisibility (Variables|Default|GetWidget) "Visible"))

(event EventBeginPlay
  (bind _returnvalue (UserInterface|CreateWidget "/Game/Widgets/LimitWidget.LimitWidget_C" (Game|GetPlayerController 0)))
  (bind _output_get (Variables|Default|SetWidget _returnvalue))
  (UserInterface|Viewport|AddtoViewport _output_get 0)
  (Widget|SetVisibility _output_get "Hidden"))

(event Collision|EventActorBeginOverlap
  (params (OtherActor :type Actor%20Object%20Reference))
  (Utilities|Casting|CastToPlayer OtherActor)
  (Widget|SetVisibility (Variables|Default|GetWidget) "Hidden"))

(event EventTick
  (params (DeltaSeconds :type Float%20%28single-precision%29)))

(fn ConstructionScript)