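; MeteorBase is an obstacle Blueprint for a meteor that moves in response to a player entering its pull zone.
; Overlapping PullZonre stores the Player reference and enables movement.
; While enabled, Tick sets the ProjectileMovement velocity from CalculateDistanceFromPlayer, whose body is not in this file.
; When a Player leaves the zone, the meteor zeroes its velocity, stops immediately and disables movement.
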(event OnComponentBeginOverlap(PullZonre)
  (params (OverlappedComponent :type Primitive%20Component%20Object%20Reference) (OtherActor :type Actor%20Object%20Reference) (OtherComp :type Primitive%20Component%20Object%20Reference) (OtherBodyIndex :type Integer) (bFromSweep :type Boolean) (SweepResult :type Hit%20Result%20Structure%20%28by%20ref%29))
  (bind _asplayer (Utilities|Casting|CastToPlayer OtherActor))
  (Variables|Default|SetPlayerRef _asplayer)
  (Variables|Default|SetMoveToPlayer true))

(event OnComponentEndOverlap(PullZonre)
  (params (OverlappedComponent :type Primitive%20Component%20Object%20Reference) (OtherActor :type Actor%20Object%20Reference) (OtherComp :type Primitive%20Component%20Object%20Reference) (OtherBodyIndex :type Integer))
  (bind _projectilemovement (Variables|Default|GetProjectileMovement))
  (Utilities|Casting|CastToPlayer OtherActor)
  (Variables|/Script/Engine.MovementComponent|SetVelocity _projectilemovement "0, 0, 0")
  (Components|Movement|StopMovementImmediately _projectilemovement)
  (Variables|Default|SetMoveToPlayer false))

(event EventBeginPlay
  (|CallParentFunction) ; This node is disabled and will not be called.\nDrag off pins to build functionality.
)

(event Collision|EventActorBeginOverlap
  (params (OtherActor :type Actor%20Object%20Reference))
  (|CallParentFunction OtherActor) ; This node is disabled and will not be called.\nDrag off pins to build functionality.
)

(event EventTick
  (params (DeltaSeconds :type Float%20%28single-precision%29))
  (|CallParentFunction DeltaSeconds)
  (if (Variables|Default|GetMoveToPlayer)
    (bind _distance (CallFunction|CalculateDistancefromPlayer (Variables|Default|GetPlayerRef)))
    (Variables|/Script/Engine.MovementComponent|SetVelocity (Variables|Default|GetProjectileMovement) _distance)))

(fn ConstructionScript
  (|CallParentFunction))