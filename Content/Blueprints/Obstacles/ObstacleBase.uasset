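; Base Paper2D obstacle that spins, damages an overlapping PlayerDefense once, and destroys itself when no Player overlaps its UnloadBox.
; CoinDrop spawns a gold or silver coin based on Type.
; Both paths call DeathAnimation to swap the sprite for a flipbook; Tick destroys the actor on its last frame, optionally with an explosion sound.
; PullZonre tracks the Player, and a helper computes speed-scaled direction toward a target, unused here.
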(event OnComponentBeginOverlap(PullZonre)
  (params (OverlappedComponent :type Primitive%20Component%20Object%20Reference) (OtherActor :type Actor%20Object%20Reference) (OtherComp :type Primitive%20Component%20Object%20Reference) (OtherBodyIndex :type Integer) (bFromSweep :type Boolean) (SweepResult :type Hit%20Result%20Structure%20%28by%20ref%29))
  (bind _asplayer (Utilities|Casting|CastToPlayer OtherActor))
  (Variables|Default|SetPlayerRef _asplayer))

(event OnComponentEndOverlap(PullZonre)
  (params (OverlappedComponent :type Primitive%20Component%20Object%20Reference) (OtherActor :type Actor%20Object%20Reference) (OtherComp :type Primitive%20Component%20Object%20Reference) (OtherBodyIndex :type Integer))
  (Variables|Default|SetPlayerRef 0))

(event OnComponentBeginOverlap(SpriteCollision)
  (params (OverlappedComponent :type Primitive%20Component%20Object%20Reference) (OtherActor :type Actor%20Object%20Reference) (OtherComp :type Primitive%20Component%20Object%20Reference) (OtherBodyIndex :type Integer) (bFromSweep :type Boolean) (SweepResult :type Hit%20Result%20Structure%20%28by%20ref%29))
  (bind _asplayer_defense (Utilities|Casting|CastToPlayerDefense OtherActor))
  (Utilities|FlowControl|DoOnce false
    (:Completed
      (Default|TakeDamage _asplayer_defense (Variables|Default|GetDamageValue))
      (CallFunction|DeathAnimation false))))

(event OnComponentEndOverlap(SpriteCollision)
  (params (OverlappedComponent :type Primitive%20Component%20Object%20Reference) (OtherActor :type Actor%20Object%20Reference) (OtherComp :type Primitive%20Component%20Object%20Reference) (OtherBodyIndex :type Integer))
  (Utilities|Casting|CastToPlayerDefense OtherActor)
  (Utilities|FlowControl|DoOnce false) ; enters at Reset
)

(event Custom|CoinDrop
  (if (>= (Variables|Default|GetType) 5)
    (Game|SpawnActorfromClass "/Game/Blueprints/Coins/GoldCoin.GoldCoin_C" (Transformation|GetActorTransform) "Undefined" 0 0)
    (else
      (Game|SpawnActorfromClass "/Game/Blueprints/Coins/SilverCoin.SilverCoin_C" (Transformation|GetActorTransform) "Undefined" 0 0)))
  (CallFunction|DeathAnimation false))

(event EventBeginPlay
  (Sprite|SetFlipbook (Variables|Default|GetPaperFlipbook) (Variables|Default|GetDeathAnim)))

(event Collision|EventActorBeginOverlap
  (params (OtherActor :type Actor%20Object%20Reference)))

(event EventTick
  (params (DeltaSeconds :type Float%20%28single-precision%29))
  (bind _paperflipbook (Variables|Default|GetPaperFlipbook))
  (Utilities|IsValid (Utilities|Array|Get(acopy) (Collision|GetOverlappingActors (Variables|Default|GetUnloadBox) "/Game/2DSideScrollerBP/Blueprints/Player.Player_C" :!class /Script/Engine.PrimitiveComponent))
    (:Is%20Valid
      (Transformation|AddLocalRotation (Variables|Default|GetPaperSprite) (Math|Rotator|MakeRotator 0.0 (* DeltaSeconds (Variables|Default|GetSpinRate)) 0.0) false false)
      (if (Variables|Default|GetDestoryingActor)
        (if (>= (Class|PaperFlipbookComponent|GetPlaybackPositioninFrames _paperflipbook) (- (Class|PaperFlipbookComponent|GetFlipbookLengthinFrames _paperflipbook) 1))
          (if (Variables|Default|GetPlaySound)
            (bind _returnvalue (Audio|SpawnSoundatLocation "/Game/Music/Explosion.Explosion" (Transformation|GetActorLocation) "0, 0, 0" 0.2 1.0 0.0 0 0))
            (Audio|Components|Audio|Play _returnvalue 0.0))
          (Actor|DestroyActor))))
    (:Is%20Not%20Valid
      (Actor|DestroyActor))))

(fn ConstructionScript)

(fn CalculateDistancefromPlayer
  (params (NewParam :type Player%20Object%20Reference))
  (Utilities|IsValid NewParam
    (:Is%20Valid
      (return (* (Math|Vector|Normalize (- (Transformation|GetWorldLocation (Variables|/Game/2DSideScrollerBP/Blueprints/Player.Player_C|GetScene NewParam)) (Transformation|GetActorLocation))) (Variables|Default|GetMovementSpeed))))))

(fn DeathAnimation
  (params (PlaySound :type Boolean))
  (bind _paperflipbook (Variables|Default|GetPaperFlipbook))
  (Variables|Default|SetPlaySound PlaySound)
  (Rendering|SetVisibility (Variables|Default|GetPaperSprite) false false)
  (Collision|SetCollisionEnabled (Variables|Default|GetSpriteCollision) "NoCollision")
  (Rendering|SetVisibility _paperflipbook true false)
  (Components|Timeline|PlayfromStart _paperflipbook)
  (Variables|Default|SetDestoryingActor true))