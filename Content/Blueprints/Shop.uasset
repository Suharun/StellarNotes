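; Shop actor that tracks player proximity for interaction and triggers discovery text.
; TriggerText overlap calls the player's ProgressChecker to show first-discovery or already-seen text, while Box overlap toggles the player's IsInteracting flag.
; Tick destroys the shop whenever no Player overlaps UnloadBox, acting as distance-based unloading.
; The construction script feeds Spline points 0 and 2 into InterpToMovement as its movement path.
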(event OnComponentBeginOverlap(TriggerText)
  (params (OverlappedComponent :type Primitive%20Component%20Object%20Reference) (OtherActor :type Actor%20Object%20Reference) (OtherComp :type Primitive%20Component%20Object%20Reference) (OtherBodyIndex :type Integer) (bFromSweep :type Boolean) (SweepResult :type Hit%20Result%20Structure%20%28by%20ref%29))
  (bind _asplayer (Utilities|Casting|CastToPlayer OtherActor))
  (if (Variables|/Game/Blueprints/ProgressChecker.ProgressChecker_C|GetShopDiscovered? (Variables|/Game/2DSideScrollerBP/Blueprints/Player.Player_C|GetProgressCheckerRef _asplayer))
    (Default|ShopSeenText (Variables|/Game/2DSideScrollerBP/Blueprints/Player.Player_C|GetProgressCheckerRef _asplayer))
    (else
      (Default|ShopDiscoveredText (Variables|/Game/2DSideScrollerBP/Blueprints/Player.Player_C|GetProgressCheckerRef _asplayer)))))

(event OnComponentBeginOverlap(Box)
  (params (OverlappedComponent :type Primitive%20Component%20Object%20Reference) (OtherActor :type Actor%20Object%20Reference) (OtherComp :type Primitive%20Component%20Object%20Reference) (OtherBodyIndex :type Integer) (bFromSweep :type Boolean) (SweepResult :type Hit%20Result%20Structure%20%28by%20ref%29))
  (bind _asplayer (Utilities|Casting|CastToPlayer OtherActor))
  (Variables|/Game/2DSideScrollerBP/Blueprints/Player.Player_C|SetIsInteracting _asplayer true))

(event OnComponentEndOverlap(Box)
  (params (OverlappedComponent :type Primitive%20Component%20Object%20Reference) (OtherActor :type Actor%20Object%20Reference) (OtherComp :type Primitive%20Component%20Object%20Reference) (OtherBodyIndex :type Integer))
  (bind _asplayer (Utilities|Casting|CastToPlayer OtherActor))
  (Variables|/Game/2DSideScrollerBP/Blueprints/Player.Player_C|SetIsInteracting _asplayer false))

(event EventBeginPlay)

(event Collision|EventActorBeginOverlap
  (params (OtherActor :type Actor%20Object%20Reference)))

(event EventTick
  (params (DeltaSeconds :type Float%20%28single-precision%29))
  (Utilities|IsValid (Utilities|Array|Get(acopy) (Collision|GetOverlappingActors (Variables|Default|GetUnloadBox) "/Game/2DSideScrollerBP/Blueprints/Player.Player_C" :!class /Script/Engine.PrimitiveComponent))
    (:Is%20Not%20Valid
      (Actor|DestroyActor))))

(fn ConstructionScript
  (bind _spline (Variables|Default|GetSpline))
  (Variables|/Script/Engine.InterpToMovementComponent|SetControlPoints (Variables|Default|GetInterpToMovement) (Utilities|Array|MakeArray (Utilities|Struct|MakeInterpControlPoint (Spline|GetLocationatSplinePoint _spline 0 "Local") true) (Utilities|Struct|MakeInterpControlPoint (Spline|GetLocationatSplinePoint _spline 2 "Local") true))))